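; BP_Door is an interactable swinging door that, when unlocked, opens on interact and automatically closes after a short delay.
; A dot product between the door's forward vector and the direction to the player picks the swing sign.
; A Timeline lerps the Arrow component's yaw to that angle, then plays in reverse to close.
; The construction script tints the Cube through a dynamic material instance using PickupColor.
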(event `/Game/Interfaces/Interface_Interact.INT_Interact`
  (params (PlayerRef :type "/Game/Player/BP_PlayerChar Object Reference"))
  ;[1 1 1] Door Open/Close
  (if (`self.isUnlocked`)
    (bind _returnvalue (`self.UpdateDoorAngle` PlayerRef))
    (bind (_direction _alpha) (`Timeline|Timeline` :!via `PlayFromStart` :!label _label)
      (:`Update`
        (`SceneComponent.K2_SetRelativeRotation` (`self.Arrow`) (`KismetMathLibrary.MakeRotator` 0.0 0.0 (`KismetMathLibrary.Lerp` 0.0 _returnvalue _alpha)) false false))
      (:`Finished`
        (if (`|EnumEquality` _direction "Forward")
          (`KismetSystemLibrary.Delay` 1.0)
          (`self.ReverseTimeline`))))))

(event `ReverseTimeline`
  ;[1 1 1] Door Open/Close
  (goto _label :!via `ReverseFromEnd`))

(fn `UpdateDoorAngle`
  (params (self2 :type "Actor Object Reference"))
  (returns (ReturnValue :type "Float (double-precision)"))
  (return (`KismetMathLibrary.Conv_IntToDouble` (`KismetMathLibrary.SelectInt` -90 90 (> (`KismetMathLibrary.Dot_VectorVector` (`KismetMathLibrary.GetDirectionUnitVector` (`self.K2_GetActorLocation`) (`self.K2_GetActorLocation` self2)) (`self.GetActorForwardVector`)) 0.0)))))

(fn `UserConstructionScript`
  (bind _returnvalue (`PrimitiveComponent.CreateDynamicMaterialInstance` (`self.Cube`) 0 "/Game/Interactables/AnimatedInteractables/MAT_Color.MAT_Color" "None"))
  (bind _output_get (set `self.ColorDMI` _returnvalue))
  (`MaterialInstanceDynamic.SetVectorParameterValue` _output_get "Color" (`self.PickupColor`)))