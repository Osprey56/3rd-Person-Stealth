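; Enemy turret that tracks and shoots at the player while they are inside its Box trigger.
; Box overlap with BP_PlayerChar starts two fast looping timers by function name, and leaving the box clears both.
; The follow timer snaps the pivot to a look-at rotation toward player 0.
; The fire timer spawns a BP_TurretProj at the ProjSpawn transform on every tick of that timer.
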(event `Fire At Player`
  ;[1 1 1] Turret Fire Action
  (`|SpawnActorFromClass` "/Game/Enemies/Turret/BP_TurretProj.BP_TurretProj_C" (`SceneComponent.K2_GetComponentToWorld` (`self.ProjSpawn`)) "Undefined" "MultiplyWithRoot" null null))

(event `Follow Player`
  ;[1 1 1] Turret Follow Action
  (`SceneComponent.K2_SetWorldRotation` (`self.Piviot`) (`KismetMathLibrary.FindLookAtRotation` (`self.K2_GetActorLocation`) (`self.K2_GetActorLocation` (`GameplayStatics.GetPlayerCharacter` 0))) false false))

(event `self.Box.OnComponentBeginOverlap`
  (params (OverlappedComponent :type "PrimitiveComponent Object Reference") (OtherActor :type "Actor Object Reference") (OtherComp :type "PrimitiveComponent Object Reference") (OtherBodyIndex :type Integer) (bFromSweep :type Boolean) (SweepResult :type "HitResult Structure (by ref)"))
  ;[1 1 1] Turret Follow / Fire At Player
  (cast `/Game/Player/BP_PlayerChar` OtherActor)
  (`KismetSystemLibrary.K2_SetTimer` null "Follow Player" 0.05 true)
  (`KismetSystemLibrary.K2_SetTimer` null "Fire At Player" 0.05 true))

(event `self.Box.OnComponentEndOverlap`
  (params (OverlappedComponent :type "PrimitiveComponent Object Reference") (OtherActor :type "Actor Object Reference") (OtherComp :type "PrimitiveComponent Object Reference") (OtherBodyIndex :type Integer))
  ;[1 1 1] Turret Follow / Fire At Player
  (cast `/Game/Player/BP_PlayerChar` OtherActor)
  (`KismetSystemLibrary.K2_ClearTimer` null "Follow Player")
  (`KismetSystemLibrary.K2_ClearTimer` null "Fire At Player"))

(fn `UserConstructionScript`)